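; YusufStar character Blueprint handling look, movement, run and jump input, plus smoothed camera collision.
; Movement input is stored, halved unless running, and exposed through GetCharacterValues with jump and weapon state, rather than applied directly.
; Each tick eases actor yaw toward control rotation while either input axis is positive.
; A reverse sphere trace drives spring arm length, interpolated at a speed scaled by camera-to-impact distance.
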(event `self.ReceiveTick`
  (params (DeltaSeconds :type "Float (single-precision)"))
  (`self.RotateCharacter` DeltaSeconds)
  (`self.Smooth Camera Collision`))

(event `EnhancedInput|/Game/YusufStar/Blueprint/Input/Actions/IA_Look`
  (params (ActionValue :type "Vector2D Structure") (ElapsedSeconds :type "Float (double-precision)") (TriggeredSeconds :type "Float (double-precision)") (InputAction :type "InputAction Object Reference" :default "/Game/YusufStar/Blueprint/Input/Actions/IA_Look.IA_Look"))
  ;[1 0.7598 0.2503] Basic Movement System
  (:`Triggered`
    (`self.AddControllerYawInput` ActionValue_X)
    (`self.AddControllerPitchInput` (* ActionValue_Y -1.0))))

(event `EnhancedInput|/Game/YusufStar/Blueprint/Input/Actions/IA_Movement`
  (params (ActionValue :type "Vector2D Structure") (ElapsedSeconds :type "Float (double-precision)") (TriggeredSeconds :type "Float (double-precision)") (InputAction :type "InputAction Object Reference" :default "/Game/YusufStar/Blueprint/Input/Actions/IA_Movement.IA_Movement"))
  ;[1 0.7598 0.2503] Basic Movement System
  (:`Triggered`
    (set `self.MovementInput` ActionValue))
  (:`Completed`
    (set `self.MovementInput` (0.0 0.0))))

(event `EnhancedInput|/Game/YusufStar/Blueprint/Input/Actions/IA_Run`
  (params (ActionValue :type Boolean) (ElapsedSeconds :type "Float (double-precision)") (TriggeredSeconds :type "Float (double-precision)") (InputAction :type "InputAction Object Reference" :default "/Game/YusufStar/Blueprint/Input/Actions/IA_Run.IA_Run"))
  ;[1 0.7598 0.2503] Basic Movement System
  (:`Triggered`
    (set `self.IsRunning` true))
  (:`Completed`
    (set `self.IsRunning` false)))

(event `EnhancedInput|/Game/YusufStar/Blueprint/Input/Actions/IA_Jump`
  (params (ActionValue :type Boolean) (ElapsedSeconds :type "Float (double-precision)") (TriggeredSeconds :type "Float (double-precision)") (InputAction :type "InputAction Object Reference" :default "/Game/YusufStar/Blueprint/Input/Actions/IA_Jump.IA_Jump"))
  ;[1 0.7598 0.2503] Basic Movement System
  (:`Triggered`
    (`self.Jump`))
  (:`Completed`
    (`self.StopJumping`)))

(event `Smooth Camera Collision`
  (bind _outhit (`KismetSystemLibrary.SphereTraceSingle` (+ (`SceneComponent.K2_GetComponentLocation` (`self.SpringArm`)) (* (`KismetMathLibrary.Normal` (- (`SceneComponent.K2_GetComponentLocation` (`self.Camera`)) (`SceneComponent.K2_GetComponentLocation` (`self.SpringArm`)))) (`self.Default Spring Arm Length`))) (`SceneComponent.K2_GetComponentLocation` (`self.SpringArm`)) (`self.Probe Radius`) "TraceTypeQuery2" false (`|MakeArray` self :!type "Actor Object Reference") "ForOneFrame"))
  (bind (_bblockinghit _binitialoverlap _time _distance _location _impactpoint) (`GameplayStatics.BreakHitResult` _outhit))
  (if _bblockinghit
    (bind _output_get (set `self.Camera Impact Point` _impactpoint))
    (set `SpringArmComponent.TargetArmLength` (`KismetMathLibrary.FInterpTo` (`SpringArmComponent.TargetArmLength` (`self.SpringArm`)) (- (`KismetMathLibrary.Vector_Distance` (`SceneComponent.K2_GetComponentLocation` (`self.SpringArm`)) _output_get) (`self.Probe Radius`)) (`GameplayStatics.GetWorldDeltaSeconds`) (`self.Camera Get Interp Speed`)) (`self.SpringArm`))
    (elif (not (`KismetMathLibrary.NearlyEqual_FloatFloat` (`SpringArmComponent.TargetArmLength` (`self.SpringArm`)) (`self.Default Spring Arm Length`) 1.0))
      (set `SpringArmComponent.TargetArmLength` (`KismetMathLibrary.FInterpTo` (`SpringArmComponent.TargetArmLength` (`self.SpringArm`)) (`self.Default Spring Arm Length`) (`GameplayStatics.GetWorldDeltaSeconds`) (`self.Camera Get Interp Speed`)) (`self.SpringArm`)))))

(fn `Camera Get Interp Speed`
  (returns (`Interp Speed` :type "Float (double-precision)"))
  (bind _camera_interp_speed (`self.Camera Interp Speed`))
  (return (`KismetMathLibrary.MapRangeClamped` (`KismetMathLibrary.Vector_Distance` (`SceneComponent.K2_GetComponentLocation` (`self.Camera`)) (`self.Camera Impact Point`)) 50.0 (`self.Default Spring Arm Length`) _camera_interp_speed (* _camera_interp_speed 10.0))))

(fn `GetCharacterValues`
  (returns (`Movement 2D` :type "Vector2D Structure") (`Is Running` :type Boolean) (`Is Jumping` :type Boolean) (`Current Weapon` :type "/Game/YusufStar/Blueprint/Data/Enum/E_WeaponTypes Enum"))
  (return (`self.Normalize Movement Input`) (`self.IsRunning`) (`NavMovementComponent.IsFalling` (`self.CharacterMovement`)) (`self.CurrentWeaponType`)))

(fn `Normalize Movement Input`
  (returns (Result :type "Vector2D Structure"))
  (bind (_movementinput_x _movementinput_y) (`KismetMathLibrary.BreakVector2D` (`self.MovementInput`)))
  (bind _returnvalue (`KismetMathLibrary.SelectFloat` 1.0 0.5 (`self.IsRunning`)))
  (return (`KismetMathLibrary.MakeVector2D` (* _movementinput_x _returnvalue) (* _movementinput_y _returnvalue))))

(fn `RotateCharacter`
  (params (DeltaTime :type "Float (single-precision)"))
  (bind (_returnvalue_roll _returnvalue_pitch) (`KismetMathLibrary.BreakRotator` (`self.K2_GetActorRotation`)))
  (bind (_movementinput_x _movementinput_y) (`KismetMathLibrary.BreakVector2D` (`self.MovementInput`)))
  (bind (_returnvalue_roll_2 _returnvalue_pitch_2 _returnvalue_yaw) (`KismetMathLibrary.BreakRotator` (`KismetMathLibrary.RInterpTo` (`self.K2_GetActorRotation`) (`self.GetControlRotation`) DeltaTime 8.0)))
  (if (or (> _movementinput_x 0.0) (> _movementinput_y 0.0))
    (`self.K2_SetActorRotation` (`KismetMathLibrary.MakeRotator` _returnvalue_roll _returnvalue_pitch _returnvalue_yaw))
    (return)))

(fn `UserConstructionScript`)